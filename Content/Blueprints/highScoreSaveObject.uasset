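; A high score save object that holds an array of score structs and keeps it as a short leaderboard.
; AddHighScore appends a new entry, re-sorts the array, then trims it to at most four entries.
; SortSaveData orders entries highest first by selection sort, repeatedly moving the DetermineHighestScore result into a temporary array.
; DetermineLowestScore also returns the weakest entry and its index, but nothing in this file calls it.
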(fn DetermineLowestScore
  (bind _highscore_struct (Variables|Default|GethighScore%20Struct))
  (for (_array_element _array_index) _highscore_struct
    (if (== _array_index 0)
      (LocalVariables|SetLowest%20Score (.score _array_element))
      (LocalVariables|SetLowest%20index _array_index)
      (elif (< (.score _array_element) (LocalVariables|GetLowest%20Score))
        (LocalVariables|SetLowest%20Score (.score _array_element))
        (LocalVariables|SetLowest%20index _array_index))))
  (return (Utilities|Array|Get(acopy) _highscore_struct (LocalVariables|GetLowest%20index)) (LocalVariables|GetLowest%20index)))

(fn DetermineHighestScore
  (bind _highscore_struct (Variables|Default|GethighScore%20Struct))
  (for (_array_element _array_index) _highscore_struct
    (if (== _array_index 0)
      (LocalVariables|SetHighest%20Score (.score _array_element))
      (LocalVariables|Sethighest%20index _array_index)
      (elif (> (.score _array_element) (LocalVariables|GetHighest%20Score))
        (LocalVariables|SetHighest%20Score (.score _array_element))
        (LocalVariables|Sethighest%20index _array_index))))
  (return (Utilities|Array|Get(acopy) _highscore_struct (LocalVariables|Gethighest%20index)) (LocalVariables|Gethighest%20index)))

(fn SortSaveData
  (while (> (Utilities|Array|Length (Variables|Default|GethighScore%20Struct)) 0)
    (bind (_high_score_struct _high_score_index) (CallFunction|DetermineHighestScore))
    (Utilities|Array|Add (LocalVariables|GetTemp) _high_score_struct)
    (Utilities|Array|RemoveIndex (Variables|Default|GethighScore%20Struct) _high_score_index))
  (Variables|Default|SethighScore%20Struct (LocalVariables|GetTemp)))

(fn AddHighScore
  (params (new%20score :type Highscore%20Struct%20Structure))
  (bind _highscore_struct (Variables|Default|GethighScore%20Struct))
  (Utilities|Array|Add _highscore_struct new%20score)
  (CallFunction|SortSaveData)
  (Utilities|Array|Resize _highscore_struct (Math|Integer|Min(Integer) 4 (Utilities|Array|Length _highscore_struct))))