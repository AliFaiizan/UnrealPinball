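; Pinball player controller that turns input into flipper, plunger and tilt actions.
; On BeginPlay it finds the plunger and sorts flippers into left and right lists, which press and release inputs drive.
; Tilting nudges the first ball found sideways, spends a game mode tilt count and plays a direction-dependent camera shake.
; A tilt attempted with none left prints "Tilt" and blocks further flips.
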(event Custom|Detect%20flippers
  (bind _outactors (Actor|GetAllActorsOfClass "/Game/Blueprints/Flipper-BP.Flipper-BP_C"))
  (for _array_element _outactors
    (switch Utilities|FlowControl|Switch|SwitchonFlipType (Variables|/Game/Blueprints/Flipper-BP.Flipper-BP_C|GetFlipType _array_element)
      (:NewEnumerator0
        (Utilities|Array|Add (Variables|Default|GetrightFlippers) _array_element))
      (:NewEnumerator1
        (Utilities|Array|Add (Variables|Default|GetleftFlippers) _array_element)))))

(event Custom|Detect%20plunger
  (bind _outactors (Actor|GetAllActorsOfClass "/Game/Blueprints/plunger_BP.plunger_BP_C"))
  (Variables|Default|Setplunger%20ref (Utilities|Array|Get(acopy) _outactors)))

(event EventBeginPlay
  (CallFunction|DetectFlippers)
  (CallFunction|DetectPlunger))

(event EventTick
  (params (DeltaSeconds :type Float%20%28single-precision%29)))

(event Input|ActionEvents|InputActionLeft
  (params (Key :type Key%20Structure))
  (bind _leftflippers (Variables|Default|GetleftFlippers))
  (:Pressed
    (for _array_element _leftflippers
      (if (Variables|Default|Getcanflip)
        (Default|Flip _array_element))))
  (:Released
    (for _array_element_2 _leftflippers
      (Default|Flop _array_element_2))))

(event Input|ActionEvents|InputActionRight
  (params (Key :type Key%20Structure))
  (bind _rightflippers (Variables|Default|GetrightFlippers))
  (:Pressed
    (for _array_element _rightflippers
      (if (Variables|Default|Getcanflip)
        (Default|Flip _array_element))))
  (:Released
    (for _array_element_2 _rightflippers
      (Default|Flop _array_element_2))))

(event Input|ActionEvents|InputActionCharge
  (params (Key :type Key%20Structure))
  (bind _plunger_ref (Variables|Default|Getplunger%20ref))
  (:Pressed
    (Default|Charge _plunger_ref))
  (:Released
    (Default|StopCharge _plunger_ref)))

(event Input|ActionEvents|InputActionrighttilt
  (params (Key :type Key%20Structure))
  (:Pressed
    (CallFunction|Tilt "NewEnumerator0")))

(event Input|ActionEvents|InputActionlefttilt
  (params (Key :type Key%20Structure))
  (:Pressed
    (CallFunction|Tilt "NewEnumerator1")))

(fn ConstructionScript)

(fn Tilt
  (params (flip%20type :type FlipType%20Enum :default "NewEnumerator0"))
  (bind _returnvalue (Game|GetPlayerCameraManager 0))
  (bind _returnvalue_2 (Camera|GetCameraRotation _returnvalue))
  (if (> (Variables|/Game/Blueprints/pinballGameMode.pinballGameMode_C|Gettilt%20count (.AsPinball%20Game%20Mode (Utilities|Casting|CastTopinballGameMode (Game|GetGameMode)))) 0)
    (bind _outactors (Actor|GetAllActorsOfClass "/Game/Blueprints/Ball-BP.Ball-BP_C"))
    (if (> (Utilities|Array|Length _outactors) 0)
      (Physics|AddImpulse (Variables|/Game/Blueprints/Ball-BP.Ball-BP_C|GetBall (Utilities|Array|Get(acopy) _outactors)) (Utilities|Select :Index flip%20type :NewEnumerator0 "-500.000000, 0, 0" :NewEnumerator1 "500.000000, 0, 0") "None" true)
      (Math|Integer|DecrementInt (Variables|/Game/Blueprints/pinballGameMode.pinballGameMode_C|Gettilt%20count (.AsPinball%20Game%20Mode (Utilities|Casting|CastTopinballGameMode (Game|GetGameMode))))
        (:%20%20
          (Class|PlayerController|ClientPlayCameraShake "/Game/Blueprints/tiltshake.tiltshake_C" 1.0 "UserDefined" (Utilities|Select :Index flip%20type :NewEnumerator0 _returnvalue_2 :NewEnumerator1 (Math|Rotator|CombineRotators _returnvalue_2 "0,180.000000, 0"))))))
    (else
      (Variables|Default|Setcanflip false)
      (Development|PrintString "Tilt"))))