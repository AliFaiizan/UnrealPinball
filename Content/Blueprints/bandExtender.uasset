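; bandExtender is a construction-script Blueprint that builds two facing posts with a stretched mesh, presumably the band, between them.
; It turns Post1 toward PostLocation and adds Post2 there with the same mesh, facing back.
; A third mesh component takes Post1's transform, with X scale set to the post distance divided by 100 so it spans the gap.
; The event graph holds only unused stubs.
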(event EventBeginPlay)

(event Collision|EventActorBeginOverlap
  (params (OtherActor :type Actor%20Object%20Reference)))

(event EventTick
  (params (DeltaSeconds :type Float%20%28single-precision%29)))

(fn ConstructionScript
  (bind _post_1 (Variables|Default|GetPost%201))
  (bind _post_location (Variables|Default|Getpost%20location))
  (bind _post_1_2 (Variables|Default|GetPost%201))
  (bind _returnvalue (Transformation|GetRelativeTransform _post_1))
  (Transformation|SetRelativeRotation _post_1_2 (Math|Rotator|FindLookatRotation (Variables|/Script/Engine.SceneComponent|GetRelativeLocation _post_1_2) (Variables|Default|Getpost%20location)) false false)
  (bind _returnvalue_2 (AddComponent|AddStaticMeshComponent false (Math|Transform|MakeTransform _post_location (Math|Rotator|FindLookatRotation _post_location (Variables|/Script/Engine.SceneComponent|GetRelativeLocation (Variables|Default|GetPost%201))) "1,1,1")))
  (bind _output_get (Variables|Default|Setpost2 _returnvalue_2))
  (Components|StaticMesh|SetStaticMesh _output_get (Variables|/Script/Engine.StaticMeshComponent|GetStaticMesh (Variables|Default|GetPost%201)))
  (AddComponent|AddStaticMeshComponent false (Math|Transform|MakeTransform (.location _returnvalue) (.rotation _returnvalue) (Math|Vector|MakeVector (/ (Math|Vector|VectorLength (- (Variables|/Script/Engine.SceneComponent|GetRelativeLocation _post_1) (Variables|Default|Getpost%20location))) 1e+02) (.y (.scale _returnvalue)) (.z (.scale _returnvalue))))))