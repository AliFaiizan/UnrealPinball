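; A pinball drop target that sinks when hit and pops back up on reset.
; Hit slides the target component down, plays a bell, disables its collision and fires the OnDrop dispatcher.
; ResetTarget restores position and collision, bound at BeginPlay to the game mode's reset and the first DropTargetSet found in the level.
; The construction script sets the target's text label from DropText.
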(event Custom|Drop
  (Components|MoveComponentTo (Variables|Default|Getdrop%20target) "0, 0,-130.000000" "0, 0, 0" false false 0.1 false)
  (Audio|PlaySound2D "/Game/Assets/Sound/Pinball_Bell01.Pinball_Bell01" 1.0 1.0 0.0 0 0)
  (Collision|SetCollisionEnabled (Variables|Default|Getdrop%20target) "NoCollision"))

(event Custom|Reset%20Target
  (Components|MoveComponentTo (Variables|Default|Getdrop%20target) "0, 0, 0" "0, 0, 0" false false 0.2 false)
  (Collision|SetCollisionEnabled (Variables|Default|Getdrop%20target) "QueryAndPhysics"))

(event EventBeginPlay
  (bind _outactors (Actor|GetAllActorsOfClass "/Game/Blueprints/DropTargetSet.DropTargetSet_C"))
  (bind _aspinball_game_mode (Utilities|Casting|CastTopinballGameMode (Game|GetGameMode)))
  (EventDispatchers|BindEventtoOnGameReset _aspinball_game_mode (delegate Custom|Reset%20Target))
  (EventDispatchers|BindEventtoResetAllTargets (Utilities|Array|Get(acopy) _outactors) (delegate Custom|Reset%20Target)))

(event Collision|EventActorBeginOverlap
  (params (OtherActor :type Actor%20Object%20Reference)))

(event EventTick
  (params (DeltaSeconds :type Float%20%28single-precision%29)))

(event Collision|EventHit
  (params (MyComp :type Primitive%20Component%20Object%20Reference) (Other :type Actor%20Object%20Reference) (OtherComp :type Primitive%20Component%20Object%20Reference) (bSelfMoved :type Boolean) (HitLocation :type Vector :default "0, 0, 0") (HitNormal :type Vector :default "0, 0, 0") (NormalImpulse :type Vector :default "0, 0, 0") (Hit :type Hit%20Result%20Structure%20%28by%20ref%29))
  (CallFunction|Drop)
  (Default|CallOnDrop))

(fn ConstructionScript
  (Rendering|Components|TextRender|SetText (Variables|Default|Gettext) (Variables|Default|Getdrop%20text)))