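; MorphTarget is a pinball slingshot bumper that kicks the ball away and awards points on contact.
; When a Ball-BP overlaps it, it applies a velocity-change impulse opposite the collision component's forward vector, plays an attached hit sound and adds score through pinballGameMode.
; A timeline drives the "sling time" scalar parameter on the Band's materials, with a dynamic material instance created in the construction script, animating the hit through the material.
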(event EventBeginPlay)

(event Collision|EventActorBeginOverlap
  (params (OtherActor :type Actor%20Object%20Reference))
  (bind _asball__bp (Utilities|Casting|CastToBall-BP OtherActor))
  (Physics|AddImpulse (Variables|/Game/Blueprints/Ball-BP.Ball-BP_C|GetBall _asball__bp) (* (Math|Vector|GetForwardVector (Variables|Default|Getcollion)) -5e+03) "None" true)
  (Audio|SpawnSoundAttached "/Game/Assets/Sound/bumperhitcue.bumperhitcue" (Variables|Default|Getband) "None" "0, 0, 0" "0, 0, 0" "KeepRelativeOffset" false 3.0 1.0 0.0 0 0)
  (bind _aspinball_game_mode (Utilities|Casting|CastTopinballGameMode (Game|GetGameMode)))
  (Default|CalculateScore _aspinball_game_mode 2e+01)
  (bind _slingtime (Timeline|Timeline_0 PlayFromStart)
    (:Update
      (Rendering|Material|SetScalarParameterValueonMaterials (Variables|Default|Getband) "sling time" _slingtime))))

(event EventTick
  (params (DeltaSeconds :type Float%20%28single-precision%29)))

(fn ConstructionScript
  (bind _returnvalue (Rendering|Material|CreateDynamicMaterialInstance (Variables|Default|Getband) 2 0 "None" :!class /Script/Engine.PrimitiveComponent))
  (Variables|Default|Setsling%20material%20instance _returnvalue))