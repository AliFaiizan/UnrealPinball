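; Pinball game mode that runs the match from main menu through ball spawning to game over and high-score entry.
; Balls spawn at the plunger, and each ball's OnDestroyed event decrements the remaining count, then respawns or ends the game.
; Game over checks saved high scores to choose between the entry widget and main menu.
; ResetGame restores class defaults, spawns a ball and broadcasts OnGameReset.
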(event Custom|create%20widget
  (bind _returnvalue (UserInterface|CreateWidget "/Game/hud.hud_C" (Game|GetPlayerController 0)))
  (UserInterface|Viewport|AddtoViewport _returnvalue 0))

(event Custom|EndGame
  (Audio|PlaySound2D "/Game/Assets/Sound/Arcade_Enemy_Death_03_m1.Arcade_Enemy_Death_03_m1" 1.0 1.0 0.0 0 0)
  (bind _current_save_object (CallFunction|GetSaveGameData))
  (if (<= (Utilities|Array|Length (Variables|/Game/Blueprints/highScoreSaveObject.highScoreSaveObject_C|GethighScore%20Struct _current_save_object)) 3)
    (CallFunction|CreateHighScoreWidget :!label _label)
    (else
      (bind _lowest_score_struct (Default|DetermineLowestScore _current_save_object))
      (if (< (.score _lowest_score_struct) (Variables|Default|Getscore))
        (goto _label)
        (else
          (CallFunction|CreateMainMenu))))))

(event Custom|on%20ball%20destroyed
  (params (DestroyedActor :type Actor%20Object%20Reference))
  (bind _result (Math|Integer|DecrementInt (Variables|Default|Getremaining%20balls))
    (:%20%20
      (Variables|Default|Setremaining%20balls _result)
      (if (> (Variables|Default|Getremaining%20balls) 0)
        (CallFunction|SpawnBall)
        (else
          (CallFunction|EndGame))))))

(event Custom|Spawn%20ball
  (Audio|PlaySound2D "/Game/Assets/Sound/Arcade_GameStart.Arcade_GameStart" 1.0 1.0 0.0 0 0)
  (bind _outactors (Actor|GetAllActorsOfClass "/Game/Blueprints/plunger_BP.plunger_BP_C"))
  (bind _returnvalue (Game|SpawnActorfromClass "/Game/Blueprints/Ball-BP.Ball-BP_C" (Math|Transform|MakeTransform (Default|GetBallLocation (Utilities|Array|Get(acopy) _outactors)) "0, 0, 0" "1,1,1") "Undefined" 0 0))
  (Audio|PlaySound2D "/Game/Assets/Sound/Pinball_BallRelease.Pinball_BallRelease" 1.0 1.0 0.0 0 0)
  (Game|BindEventtoOnDestroyed _returnvalue (delegate Custom|on%20ball%20destroyed)))

(event Custom|create%20high%20score%20widget
  (bind _returnvalue (Game|GetPlayerController 0))
  (bind _returnvalue_2 (UserInterface|CreateWidget "/Game/highscoreEntry.highscoreEntry_C" _returnvalue))
  (UserInterface|Viewport|AddtoViewport _returnvalue_2 0)
  (Variables|/Script/Engine.PlayerController|SetbShowMouseCursor _returnvalue true))

(event Custom|Create%20main%20menu
  (bind _returnvalue (Game|GetPlayerController 0))
  (CallFunction|GetSaveGameData)
  (Viewport|RemoveAllWidgets)
  (bind _returnvalue_2 (UserInterface|CreateWidget "/Game/MainMenu.MainMenu_C" _returnvalue))
  (UserInterface|Viewport|AddtoViewport _returnvalue_2 0)
  (Variables|/Script/Engine.PlayerController|SetbShowMouseCursor _returnvalue true))

(event Custom|Reset%20game
  (bind (_multiplier _score _remaining_balls _highscoresave_name _on_game_reset _tilt_count) (Utilities|GetClassDefaults "pinballGameMode_C"))
  (Variables|Default|Setmultiplier _multiplier)
  (Variables|Default|Setscore _score)
  (Variables|Default|Setremaining%20balls _remaining_balls)
  (Variables|Default|Settilt%20count _tilt_count)
  (CallFunction|SpawnBall)
  (Default|CallOnGameReset))

(event EventBeginPlay
  (CallFunction|CreateMainMenu))

(event EventTick
  (params (DeltaSeconds :type Float%20%28single-precision%29)))

(fn ConstructionScript)

(fn CalculateScore
  (params (score :type Float%20%28single-precision%29))
  (bind _output_get (Variables|Default|Setscore (+ (Variables|Default|Getscore) (* score (Variables|Default|Getmultiplier)))))
  (return _output_get))

(fn GetSaveGameData
  (bind _highscore_save (Variables|Default|Gethighscore%20save)
    (:then
      (return _highscore_save))
    (:else
      (bind _returnvalue (SaveGame|DoesSaveGameExist (Variables|Default|Gethighscoresave%20name)))
      (if _returnvalue
        (bind _returnvalue_2 (SaveGame|LoadGamefromSlot (Variables|Default|Gethighscoresave%20name)))
        (bind _ashigh_score_save_object (Utilities|Casting|CastTohighScoreSaveObject _returnvalue_2))
        (Default|SortSaveData _ashigh_score_save_object)
        (bind _output_get (Variables|Default|Setcurrent%20save%20object _ashigh_score_save_object))
        (return _output_get)
        (else
          (bind _returnvalue_3 (SaveGame|CreateSaveGameObject "/Game/Blueprints/highScoreSaveObject.highScoreSaveObject_C"))
          (bind _output_get_2 (Variables|Default|Setcurrent%20save%20object _returnvalue_3))
          (return _output_get_2))))))