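; Pinball drop target set that raises the game mode's multiplier when all its lettered targets are dropped.
; The construction script spawns one DropTarget child actor per character of an uppercased string, spacing them evenly by the distance between two posts.
; Target drop events are bound to count down; at zero a bell plays and all targets reset after a delay.
; The game mode's reset event restores the counter to the string length.
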(event Custom|Process%20Drop%20Target
  (bind _result (Math|Integer|DecrementInt (Variables|Default|GetDropTargetCounter))
    (:%20%20
      (if (== _result 0)
        (Audio|PlaySound2D "/Game/Assets/Sound/Bell_Impact01.Bell_Impact01" 1.0 1.0 0.0 0 0)
        (bind _aspinball_game_mode (Utilities|Casting|CastTopinballGameMode (Game|GetGameMode)))
        (Math|Float|IncrementFloat (Variables|/Game/Blueprints/pinballGameMode.pinballGameMode_C|Getmultiplier _aspinball_game_mode)
          (:%20%20
            (Utilities|FlowControl|Delay 2.0)
            (Default|CallResetAllTargets)))))))

(event Custom|Reset%20drop%20target%20set
  (Variables|Default|SetDropTargetCounter (Utilities|String|Len (Variables|Default|Gettext%20string))))

(event EventBeginPlay
  (|CallParentFunction)
  (bind _aspinball_game_mode (Utilities|Casting|CastTopinballGameMode (Game|GetGameMode)))
  (EventDispatchers|BindEventtoOnGameReset _aspinball_game_mode (delegate Custom|Reset%20drop%20target%20set)))

(event Collision|EventActorBeginOverlap
  (params (OtherActor :type Actor%20Object%20Reference))
  (|CallParentFunction OtherActor) ; This node is disabled and will not be called.\nDrag off pins to build functionality.
)

(event EventTick
  (params (DeltaSeconds :type Float%20%28single-precision%29))
  (|CallParentFunction DeltaSeconds) ; This node is disabled and will not be called.\nDrag off pins to build functionality.
)

(fn ConstructionScript
  (bind _post_1 (Variables|Default|GetPost%201))
  (|CallParentFunction)
  (bind _output_get (Variables|Default|Settext%20string (Class|KismetStringLibrary|ToUpper (Variables|Default|Gettext%20string))))
  (for (_array_element _array_index) (Utilities|String|GetCharacterArrayfromString _output_get)
    (bind _returnvalue (AddComponent|AddChildActorComponent false (Math|Transform|MakeTransform (+ (* (Math|Vector|GetForwardVector _post_1) (* (+ _array_index 1) (/ (Math|Vector|VectorLength (- (Variables|/Script/Engine.SceneComponent|GetRelativeLocation (Variables|Default|GetPost%201)) (Variables|/Script/Engine.SceneComponent|GetRelativeLocation (Variables|Default|Getpost2)))) (Math|Conversions|ToFloat(Integer) (+ (Utilities|Array|Length (Utilities|String|GetCharacterArrayfromString _output_get)) 1))))) (* (Math|Vector|GetRightVector _post_1) 20)) (Variables|/Script/Engine.SceneComponent|GetRelativeRotation (Variables|Default|GetPost%201)) "1,1,1")))
    (bind _asdrop_target (Utilities|Casting|CastToDropTarget (Variables|/Script/Engine.ChildActorComponent|GetChildActor _returnvalue)))
    (Rendering|Components|TextRender|SetText (Variables|/Game/Blueprints/DropTarget.DropTarget_C|Gettext _asdrop_target) (Utilities|Text|ToText(String) _array_element))
    (EventDispatchers|BindEventtoOnDrop _asdrop_target (EventDispatchers|CreateEvent :!event Custom|Process%20Drop%20Target))))