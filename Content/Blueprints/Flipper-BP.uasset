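; Pinball flipper actor that swings between a rest and a raised angle on Flip and Flop events.
; The construction script uses FlipType to pick mirrored start and end yaw angles, set the rest pose, and mirror the mesh on X for the right side.
; Flip eases the flipper to the end rotation with MoveComponentTo and plays a side-specific sound, while Flop eases it back silently.
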(event Custom|Flop
  (Components|MoveComponentTo (Variables|Default|GetFlipper) "0, 0, 0" (Variables|Default|GetStart%20Rotation) true false (Variables|Default|GetFlpTime) false))

(event Custom|Flip
  (Components|MoveComponentTo (Variables|Default|GetFlipper) "0, 0, 0" (Variables|Default|GetEnd%20Rotation) true false (Variables|Default|GetFlpTime) false)
  (switch Utilities|FlowControl|Switch|SwitchonFlipType (Variables|Default|GetFlipType)
    (:NewEnumerator0
      (Audio|PlaySound2D "/Game/Assets/Sound/Pinball_FlipperRight.Pinball_FlipperRight" 0.15 1.0 0.0 0 0))
    (:NewEnumerator1
      (Audio|PlaySound2D "/Game/Assets/Sound/Pinball_FlipperLeft.Pinball_FlipperLeft" 0.15 1.0 0.0 0 0))))

(event EventBeginPlay)

(event Collision|EventActorBeginOverlap
  (params (OtherActor :type Actor%20Object%20Reference)))

(event EventTick
  (params (DeltaSeconds :type Float%20%28single-precision%29)))

(fn ConstructionScript
  (Variables|Default|SetStart%20Rotation (Utilities|Select :Index (Variables|Default|GetFlipType) :NewEnumerator0 "0,-20.000000,0" :NewEnumerator1 "0,20.000000,0"))
  (Variables|Default|SetEnd%20Rotation (Utilities|Select :Index (Variables|Default|GetFlipType) :NewEnumerator0 "0,20.000000,0" :NewEnumerator1 "0,-20.000000,0"))
  (Transformation|SetRelativeRotation (Variables|Default|GetFlipper) (Variables|Default|GetStart%20Rotation) false false)
  (switch Utilities|FlowControl|Switch|SwitchonFlipType (Variables|Default|GetFlipType)
    (:NewEnumerator0
      (Transformation|SetRelativeScale3D (Variables|Default|GetFlipper) "-1.000000,1.000000,1.000000"))))