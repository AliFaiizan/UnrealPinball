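; Pinball bumper actor that knocks the ball away and awards points through the pinball game mode.
; On ball overlap it applies a radial velocity impulse, adds its score, then plays a hit sound and sparks.
; A timeline drops the bumper mechanism while raising point light intensity and material emissive boost.
; The construction script sets material and light color from the BumperColor enum and creates the dynamic material instance.
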(event EventBeginPlay)

(event Collision|EventActorBeginOverlap
  (params (OtherActor :type Actor%20Object%20Reference))
  (bind _pointlight (Variables|Default|GetPointLight))
  (bind _asball__bp (Utilities|Casting|CastToBall-BP OtherActor))
  (Physics|AddImpulse (Variables|/Game/Blueprints/Ball-BP.Ball-BP_C|GetBall _asball__bp) (* (Math|Vector|GetUnitDirection(Vector) (Transformation|GetActorLocation) (Transformation|GetActorLocation _asball__bp)) 5e+03) "None" true)
  (bind _aspinball_game_mode (Utilities|Casting|CastTopinballGameMode (Game|GetGameMode)))
  (bind _new_score (Default|CalculateScore _aspinball_game_mode (Variables|Default|Getscore)))
  (Development|PrintString (Utilities|String|ToString(Float) _new_score))
  (Audio|SpawnSoundAttached "/Game/Assets/Sound/BumperHit.BumperHit" (Variables|Default|GetBumper) "None" "0, 0, 0" "0, 0, 0" "KeepRelativeOffset" false 1.0 1.0 0.0 0 0)
  (Effects|SpawnEmitteratLocation "/Game/Meterial/bumperSparks.bumperSparks" (Transformation|GetWorldLocation (Variables|Default|GetBumper_Machanism)))
  (bind _bumpmac (Timeline|BumpMac PlayFromStart)
    (:Update
      (Transformation|SetRelativeLocation (Variables|Default|GetBumper_Machanism) (Math|Vector|Lerp(Vector) "0, 0, 0" "0, 0,-70.000000" _bumpmac) false false)
      (Rendering|Components|Light|SetLightColor _pointlight (Variables|Default|Getclr) true)
      (Rendering|Components|Light|SetIntensity _pointlight (Math|Float|Lerp 0.0 5e+03 _bumpmac))
      (Rendering|Material|SetScalarParameterValue (Variables|Default|GetBump%20MDI) "Emissive Boost" (Math|Float|Lerp 0.0 5e+01 _bumpmac) :!class /Script/Engine.MaterialInstanceDynamic))))

(event EventTick
  (params (DeltaSeconds :type Float%20%28single-precision%29)))

(fn ConstructionScript
  (bind _bumper (Variables|Default|GetBumper))
  (switch Utilities|FlowControl|Switch|Switchonbumpercolors (Variables|Default|Getbumper%20color)
    (:NewEnumerator0
      (Rendering|Material|SetMaterial _bumper 1 "/Game/Meterial/B_red_mat.B_red_mat")
      (Variables|Default|Setclr "(R=0.765625,G=0.031499,B=0.023883,A=1.000000)"))
    (:NewEnumerator1
      (Rendering|Material|SetMaterial _bumper 1 "/Game/Meterial/B_green_mat.B_green_mat")
      (Variables|Default|Setclr "(R=0.039585,G=0.932292,B=0.050743,A=1.000000)"))
    (:NewEnumerator2
      (Rendering|Material|SetMaterial _bumper 1 "/Game/Meterial/M_Bumper.M_Bumper")
      (Variables|Default|Setclr "(R=0.000000,G=0.057259,B=0.536458,A=1.000000)"))
    (:NewEnumerator3
      (Rendering|Material|SetMaterial _bumper 1 "/Game/Meterial/B_yellow_mat.B_yellow_mat")
      (Variables|Default|Setclr "(R=0.781250,G=0.743921,B=0.034102,A=1.000000)")))
  (bind _returnvalue (Rendering|Material|CreateDynamicMaterialInstance (Variables|Default|GetBumper) 1 0 "None" :!class /Script/Engine.PrimitiveComponent))
  (Variables|Default|SetBump%20MDI _returnvalue))