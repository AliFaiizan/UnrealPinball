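; Spline-driven pinball rail that scores when a ball drops off it.
; The construction script adds a spline mesh per segment, using Start, Mid and End meshes and a configurable start scale on the first.
; It also moves a trigger Box to an offset from the second-to-last spline point.
; When a Ball-BP leaves the Box, it plays a drop sound and adds points through pinballGameMode.
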(event OnComponentBeginOverlap(Box)
  (params (OverlappedComponent :type Primitive%20Component%20Object%20Reference) (OtherActor :type Actor%20Object%20Reference) (OtherComp :type Primitive%20Component%20Object%20Reference) (OtherBodyIndex :type Integer) (bFromSweep :type Boolean) (SweepResult :type Hit%20Result%20Structure%20%28by%20ref%29)))

(event OnComponentEndOverlap(Box)
  (params (OverlappedComponent :type Primitive%20Component%20Object%20Reference) (OtherActor :type Actor%20Object%20Reference) (OtherComp :type Primitive%20Component%20Object%20Reference) (OtherBodyIndex :type Integer))
  (bind _asball__bp (Utilities|Casting|CastToBall-BP OtherActor))
  (Audio|PlaySound2D _asball__bp "/Game/Assets/Sound/Pinball_BallDropFromSlide.Pinball_BallDropFromSlide" 1.0 1.0 0.0 0 0)
  (Default|CalculateScore (.AsPinball%20Game%20Mode (Utilities|Casting|CastTopinballGameMode (Game|GetGameMode))) 5e+01))

(event EventBeginPlay)

(event Collision|EventActorBeginOverlap
  (params (OtherActor :type Actor%20Object%20Reference)))

(event EventTick
  (params (DeltaSeconds :type Float%20%28single-precision%29)))

(fn ConstructionScript
  (bind _spline (Variables|Default|GetSpline))
  (bind _spline_2 (Variables|Default|GetSpline))
  (bind _returnvalue (Spline|GetNumberOfSplinePoints _spline))
  (bind _returnvalue_2 (- _returnvalue 2))
  (for _index (range 0 _returnvalue_2)
    (bind _returnvalue_3 (AddComponent|AddSplineMeshComponent false))
    (if (== _index 0)
      (Components|StaticMesh|SetStaticMesh _returnvalue_3 (Variables|Default|Getstart))
      (SplineMesh|SetStartScale _returnvalue_3 (Math|Vector2D|MakeVector2D (Variables|Default|GetstartScale) 1.0) true :!class /Script/Engine.SplineMeshComponent)
      (elif (== _index _returnvalue_2)
        (Components|StaticMesh|SetStaticMesh _returnvalue_3 (Variables|Default|Getend))
        (Transformation|SetRelativeLocation (Variables|Default|GetBox) (+ (Spline|GetLocationatSplinePoint (Variables|Default|GetSpline) _index "Local") "70.000000, 0,30.000000") false false)
        (else
          (Components|StaticMesh|SetStaticMesh _returnvalue_3 (Variables|Default|Getmid)))))
    (SplineMesh|SetStartandEnd _returnvalue_3 (.Location (Spline|GetLocationandTangentatSplinePoint _spline_2 _index "Local")) (.Tangent (Spline|GetLocationandTangentatSplinePoint _spline_2 _index "Local")) (.Location (Spline|GetLocationandTangentatSplinePoint _spline_2 (+ _index 1) "Local")) (.Tangent (Spline|GetLocationandTangentatSplinePoint _spline_2 (+ _index 1) "Local")) true :!class /Script/Engine.SplineMeshComponent)))