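; Force-direction volume that steers balls along its Arrow component while they are inside its Box.
; Each tick, it converts every overlapping ball's physics velocity into the Arrow's local space.
; It rapidly interpolates that toward a forward-only velocity with clamped minimum and maximum speed, damping sideways motion.
; The result is converted back to world space and replaces the ball's linear velocity.
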(event EventBeginPlay)

(event Collision|EventActorBeginOverlap
  (params (OtherActor :type Actor%20Object%20Reference)))

(event EventTick
  (params (DeltaSeconds :type Float%20%28single-precision%29))
  (bind _arrow (Variables|Default|GetArrow))
  (bind _returnvalue (Transformation|GetWorldTransform _arrow))
  (for _array_element (Collision|GetOverlappingActors (Variables|Default|GetBox) "/Game/Blueprints/Ball-BP.Ball-BP_C" :!class /Script/Engine.PrimitiveComponent)
    (Physics|SetPhysicsLinearVelocity (Variables|/Game/Blueprints/Ball-BP.Ball-BP_C|GetBall (.AsBall-%20BP (Utilities|Casting|CastToBall-BP _array_element))) (Math|Transform|TransformDirection _returnvalue (Math|Interpolation|VInterpTo (Math|Transform|InverseTransformDirection _returnvalue (Transformation|GetComponentVelocity (Variables|/Game/Blueprints/Ball-BP.Ball-BP_C|GetBall (.AsBall-%20BP (Utilities|Casting|CastToBall-BP _array_element))))) (Math|Vector|MakeVector (Math|Float|Clamp(Float) (.X (Math|Vector|BreakVector (Math|Transform|InverseTransformDirection _returnvalue (Transformation|GetComponentVelocity (Variables|/Game/Blueprints/Ball-BP.Ball-BP_C|GetBall (.AsBall-%20BP (Utilities|Casting|CastToBall-BP _array_element))))))) 5e+02 1e+04) 0.0 0.0) (Utilities|Time|GetWorldDeltaSeconds) 1e+02)) false "None")))

(fn ConstructionScript)