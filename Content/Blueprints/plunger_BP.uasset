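; Pinball plunger actor that pulls back while charging and snaps forward on release.
; Charge plays a timeline that lerps the Plunger component back along its relative negative Y axis.
; StopCharge halts the timeline, plays the ball launch sound and quickly returns the plunger with MoveComponentTo.
; GetBallLocation converts a local ball offset to world space through the plunger's transform, so the point follows its movement.
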(event Custom|Charge
  (bind _chargealpha (Timeline|Chargetimeline PlayFromStart)
    (:Update
      (Transformation|SetRelativeLocation (Variables|Default|Getplunger) (Math|Vector|Lerp(Vector) "0, 0, 0" "0,-300.000000, 0" _chargealpha) false false))))

(event Custom|Stop%20Charge
  (Utilities|FlowControl|Sequence
    (:then_0
      (bind _chargealpha (Timeline|Chargetimeline Stop)
        (:Update
          (Transformation|SetRelativeLocation (Variables|Default|Getplunger) (Math|Vector|Lerp(Vector) "0, 0, 0" "0,-300.000000, 0" _chargealpha) false false))))
    (:then_1
      (Audio|PlaySound2D "/Game/Assets/Sound/Pinball_BallLaunch.Pinball_BallLaunch" 1.0 1.0 0.0 0 0)
      (Components|MoveComponentTo (Variables|Default|Getplunger) "0, 0, 0" "0, 0, 0" false false 0.08 false))))

(event EventBeginPlay)

(event Collision|EventActorBeginOverlap
  (params (OtherActor :type Actor%20Object%20Reference)))

(event EventTick
  (params (DeltaSeconds :type Float%20%28single-precision%29)))

(fn ConstructionScript)

(fn GetBallLocation
  (return (Math|Transform|TransformLocation (Transformation|GetWorldTransform (Variables|Default|Getplunger)) (Variables|Default|Getball%20location))))